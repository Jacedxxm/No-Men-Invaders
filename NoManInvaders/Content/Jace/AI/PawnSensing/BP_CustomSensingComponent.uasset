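; A custom AI sight component that checks whether its owner can see player pawn 0 and writes the result to the Blackboard key CanSeeTarget.
; A looping timer runs the check at a set interval and can be stopped.
; Sight requires an unblocked Visibility line trace to the player, within range and inside a forward cone tested by dot-product angle.
; A Debug flag draws the cone and prints failure reasons.
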(event `self.ReceiveBeginPlay`
  (set `self.TargetPawn` (`GameplayStatics.GetPlayerPawn` 0))
  (`self.Begin Sensing`))

(event `Begin Sensing`
  (bind _returnvalue (`KismetSystemLibrary.K2_SetTimerDelegate` (delegate `Sense`) (`self.SensingInterval`) true))
  (set `self.SensingTimerRef` _returnvalue))

(event `Stop Sensing`
  (`KismetSystemLibrary.K2_ClearAndInvalidateTimerHandle` (`self.SensingTimerRef`)))

(event `Sense`
  (bind _cansee_1 (`self.SenseForTarget`))
  (`/Game/Jace/AI/FunctionLibrary/BFL_AI.UpdateBBKey` (`AIBlueprintHelperLibrary.GetAIController` (`self.GetOwner`)) "CanSeeTarget" "NewEnumerator0" _cansee_1))

(fn `DebugMex`
  (params (InString :type String))
  (if (`self.Debug?`)
    (`KismetSystemLibrary.PrintString` InString)))

(fn `SenseForTarget`
  (returns (`CanSee?1` :type Boolean))
  (locals (`CanSee?` :type Boolean))
  (bind _returnvalue_location (`KismetMathLibrary.BreakTransform` (`self.K2_GetComponentToWorld`)))
  (bind _pawnsensingconeangle (`self.PawnSensingConeAngle`))
  (bind (_currenthitresult_bblockinghit _currenthitresult_binitialoverlap _currenthitresult_time _currenthitresult_distance) (`GameplayStatics.BreakHitResult` (`self.CurrentHitResult`)))
  (bind (_currenthitresult_bblockinghit_2 _currenthitresult_binitialoverlap_2 _currenthitresult_time_2 _currenthitresult_distance_2 _currenthitresult_location _currenthitresult_impactpoint _currenthitresult_normal _currenthitresult_impactnormal _currenthitresult_physmat _currenthitresult_hitactor) (`GameplayStatics.BreakHitResult` (`self.CurrentHitResult`)))
  (bind _returnvalue (`KismetMathLibrary.DegAcos` (`KismetMathLibrary.Dot_VectorVector` (`self.GetForwardVector`) (`KismetMathLibrary.GetDirectionUnitVector` (`self.K2_GetComponentLocation`) (`Actor.K2_GetActorLocation` (`self.TargetPawn`))))))
  (set `local.CanSee?` false)
  (if (`self.Debug?`)
    (`KismetSystemLibrary.DrawDebugConeInDegrees` _returnvalue_location (`self.GetForwardVector`) (`self.PawnSensingRange`) _pawnsensingconeangle _pawnsensingconeangle 12 (struct :`R` 1.0 :`G` 1.0 :`B` 1.0 :`A` 1.0) (`self.SensingInterval`) 5.0))
  (bind (_outhit _returnvalue_2) (`KismetSystemLibrary.LineTraceSingle` (`self.K2_GetComponentLocation`) (`Actor.K2_GetActorLocation` (`self.TargetPawn`)) "TraceTypeQuery1" false (`|MakeArray` (`self.GetOwner`)) (`self.TraceDebugType`)))
  (if _returnvalue_2
    (set `self.CurrentHitResult` _outhit)
    (if (== _currenthitresult_hitactor (`self.TargetPawn`))
      (if (<= _currenthitresult_distance (`self.PawnSensingRange`))
        (if (<= _returnvalue (`self.PawnSensingConeAngle`))
          (set `local.CanSee?` true)
          (return (`local.CanSee?`))
          (else
            (`self.DebugMex` (`KismetStringLibrary.Concat_StrStr` "Pawn Sensing Target Out of peripheral Vision" "Angle ==" (`KismetStringLibrary.Conv_DoubleToString` _returnvalue)))
            (return (`local.CanSee?`))))
        (else
          (`self.DebugMex` "Pawn Sensing Hit Result Was Out of Pawn Sensing Range")))
      (else
        (`self.DebugMex` "PawnSensingIsBlockedByObjects")
        (return (`local.CanSee?`))))
    (else
      (`self.DebugMex` "No Hit From Custom pawn")
      (return (`local.CanSee?`)))))