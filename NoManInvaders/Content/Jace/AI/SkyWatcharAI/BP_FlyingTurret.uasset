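; BP_FlyingTurret is a flying turret enemy driven by an AI controller and behavior tree targeting the player pawn.
; Construction creates a dynamic emissive eye material for its changing component and binds health values and a health bar widget to its health system component.
; BeginPlay sets up the controller and physics move-to parameters.
; On death it spawns an explosion, briefly delays, destroys itself and calls the enemy-destroyed notification.
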(event `self.ReceiveBeginPlay`
  (bind _asai_controller (cast `/Game/Jace/AI/BT/AI_Controller` (`AIBlueprintHelperLibrary.GetAIController` self)))
  (`/Game/Jace/AI/BT/AI_Controller.Setup AIC` _asai_controller (`self.BT`) (`GameplayStatics.GetPlayerPawn` 0))
  (`/Game/Jace/AI/Enemies/Components/BP_PhysicsMoveToParameters.Setup` (`self.BP_PhysicsMoveToParameters`)))

(event `self.BP_HealthSystemComponent.OnDead`
  (`GameplayStatics.SpawnEmitterAtLocation` "/Game/StarterContent/Particles/P_Explosion.P_Explosion" (`self.K2_GetActorLocation`))
  (`KismetSystemLibrary.Delay` 0.2)
  (`self.K2_DestroyActor`)
  (`self.OnEnemyDestroyed`))

(fn `UserConstructionScript`
  ;[1 1 1] Setup Dynamic Eye and Component
  (bind _returnvalue (`PrimitiveComponent.CreateDynamicMaterialInstance` (`self.Eye`) 0 "/Game/Jace/Materials/MM_EmissiveColor_Inst1.MM_EmissiveColor_Inst1" "None"))
  (bind _output_get (set `self.EyeDynamicMatRef` _returnvalue))
  (`/Game/Jace/AI/Enemies/TurretGuardian/BP_ChangingComponent.Setup` (`self.BP_ChangingComponent`) _output_get)
  (`/Game/Jace/Blueprints/HealthSystem/BP_HealthSystemComponent.Setup Damageable Component` (`self.BP_HealthSystemComponent`) null (`self.MaxHealth`) (`self.Health`) (`self.Widget`)))