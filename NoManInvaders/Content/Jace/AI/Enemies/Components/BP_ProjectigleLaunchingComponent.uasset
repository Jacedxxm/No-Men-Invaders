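; BP_ProjectigleLaunchingComponent is a component that fires a projectile toward a target location, intended to be called by AI behavior tree tasks or the player.
; LaunchProjectileAtLocation spawns the configured actor class at the component's transform and sets its ProjectileMovementComponent velocity along the direction to the target, scaled by ProjectileSpeed.
; A successful launch plays an explosion sound and small particle burst at the origin.
; A missing movement component only prints an error.
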(event `LaunchProjectileAtLocation`
  (params (TargetLocation :type "Vector Structure"))
  (bind _returnvalue (`self.K2_GetComponentLocation`))
  ;[1 1 1] Called From AI BTT or Player
  (set `self.TargetLocation` TargetLocation)
  ;[1 1 1] Launch Projectiles
  (bind _returnvalue_2 (`|SpawnActorFromClass` (`self.ProjectileMovement`) (`self.K2_GetComponentToWorld`) "Undefined" "MultiplyWithRoot" null null))
  (bind _returnvalue_3 (`Actor.GetComponentByClass` _returnvalue_2 "/Script/Engine.ProjectileMovementComponent"))
  (`/Engine/EditorBlueprintResources/StandardMacros.IsValid` _returnvalue_3
    (:`Is Valid`
      (set `self.ProjectileMovementComp` _returnvalue_3)
      ;[1 1 1] Velocity
      (set `MovementComponent.Velocity` (* (`KismetMathLibrary.GetDirectionUnitVector` (`self.K2_GetComponentLocation`) (`self.TargetLocation`)) (`self.ProjectileSpeed`)) (`self.ProjectileMovementComp`))
      ;[1 1 1] Feedback
      (`GameplayStatics.SpawnSoundAtLocation` "/Game/StarterContent/Audio/Explosion_Cue.Explosion_Cue" _returnvalue (struct) 1.0 1.0 0.0 null null)
      (`GameplayStatics.SpawnEmitterAtLocation` "/Game/StarterContent/Particles/P_Explosion.P_Explosion" _returnvalue (struct) (0.2 0.2 0.2) true "AutoRelease"))
    (:`Is Not Valid`
      (`KismetSystemLibrary.PrintString` "Projectile doesn't have ProjectileMovement"))))