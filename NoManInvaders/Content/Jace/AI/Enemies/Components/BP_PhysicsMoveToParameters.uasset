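; Component for AI enemies that prepares its owning Character for physics-driven movement, judging by its name as parameters for a physics move-to.
; Setup caches the owner and its capsule, turns on physics simulation for the capsule, disables gravity on both capsule and character movement, and applies linear and angular damping.
; A non-Character owner only prints a failure message that references an Add Force behavior tree task.
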(event `Setup`
  (bind _physicscapsuleref (`self.PhysicsCapsuleRef`))
  (bind _physicscapsuleref_2 (`self.PhysicsCapsuleRef`))
  (bind _ascharacter (cast `Character` (`self.GetOwner`))
    (:`then`
      (bind _output_get (set `self.OwningCharacterRef` _ascharacter))
      (set `self.PhysicsCapsuleRef` (`Character.CapsuleComponent` _output_get))
      (`PrimitiveComponent.SetSimulatePhysics` _physicscapsuleref_2 true)
      (`PrimitiveComponent.SetEnableGravity` _physicscapsuleref_2 false)
      (set `CharacterMovementComponent.GravityScale` 0.0 (`Character.CharacterMovement` (`self.OwningCharacterRef`)))
      (`PrimitiveComponent.SetLinearDamping` _physicscapsuleref (`self.LinearDamping`))
      (`PrimitiveComponent.SetAngularDamping` _physicscapsuleref (`self.AngularDamping`)))
    (:`CastFailed`
      (`KismetSystemLibrary.PrintString` "Add Force BTT Task Failed cause controlled pawn wasn't Character"))))