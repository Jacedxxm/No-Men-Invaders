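; Projectile for the Turret Guardian enemy that explodes on impact and damages whatever it hits.
; A sphere hit triggers Detonation, which runs once to spawn an explosion effect and deep-pitched sound, then destroys the actor.
; The hit actor takes damage through its BP_HealthSystemComponent, if it has one.
; A LaunchCharacter knockback function exists but is not wired to run.
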(event `self.Sphere.OnComponentHit`
  (params (HitComponent :type "PrimitiveComponent Object Reference") (OtherActor :type "Actor Object Reference") (OtherComp :type "PrimitiveComponent Object Reference") (NormalImpulse :type "Vector Structure") (Hit :type "HitResult Structure (by ref)"))
  (bind _returnvalue (`self.GetComponentByClass` OtherActor "/Game/Jace/Blueprints/HealthSystem/BP_HealthSystemComponent.BP_HealthSystemComponent_C"))
  (`self.Detonation`)
  (`/Engine/EditorBlueprintResources/StandardMacros.IsValid` OtherActor
    (:`Is Valid`
      (`/Engine/EditorBlueprintResources/StandardMacros.IsValid` _returnvalue
        (:`Is Valid`
          (`/Game/Jace/Blueprints/HealthSystem/BP_HealthSystemComponent.TakeDamageViaComponent` _returnvalue (`self.Damage`)))))))

(fn `Detonation`
  (bind _returnvalue (`self.K2_GetActorLocation`))
  (`/Engine/EditorBlueprintResources/StandardMacros.DoOnce` false
    (:`Completed`
      (`GameplayStatics.SpawnEmitterAtLocation` "/Game/StarterContent/Particles/P_Explosion.P_Explosion" _returnvalue)
      (`GameplayStatics.SpawnSoundAtLocation` "/Game/StarterContent/Audio/Explosion02.Explosion02" _returnvalue (struct) 2.0 0.3 0.0 null null)
      (`self.K2_DestroyActor`))))

(fn `LaunchCharacter`
  (params (Character :type "Actor Object Reference") (InputPin :type "Actor Object Reference"))
  (bind _ascharacter (cast `Character` InputPin))
  (`Character.LaunchCharacter` _ascharacter (* (+ (`KismetMathLibrary.GetDirectionUnitVector` (`SceneComponent.K2_GetComponentLocation` (`Actor.RootComponent` Character)) (`self.K2_GetActorLocation` Character)) (0.0 0.0 0.5)) 600.0) false false))

(fn `UserConstructionScript`)