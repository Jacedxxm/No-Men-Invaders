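; Enemy spawner actor that spawns queued enemy classes at its own transform and reports defeats to GM_Spaceship.
; AddEnemyToQueue appends a class and spawns immediately if no enemy overlaps its Sphere.
; SpawnEnemy pops the queue head, binds the enemy's destroyed event and sets a timer to call itself again.
; A looping BeginPlay timer also calls SpawnEnemy, without the overlap check.
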(event `self.ReceiveBeginPlay`
  (`KismetSystemLibrary.K2_SetTimerDelegate` (delegate `TryToSpawn`) 2.0 true))

(event `TryToSpawn`
  (`self.SpawnEnemy`))

(event `OnEnemyDefeated`
  (bind _asgm_spaceship (cast `/Game/Jace/Blueprints/GameModes/GM_Spaceship` (`GameplayStatics.GetGameMode`)))
  (`/Game/Jace/Blueprints/GameModes/GM_Spaceship.OnEnemyDefeated` _asgm_spaceship))

(fn `AddEnemyToQueue`
  (params (EnemyClass :type "/Game/Jace/AI/SkyWatcharAI/BP_FlyingTurret Class Reference (by ref)"))
  (`KismetArrayLibrary.Array_Add` (`self.EnemyQueue`) EnemyClass)
  (if (not (`KismetArrayLibrary.Array_IsValidIndex` (`PrimitiveComponent.GetOverlappingActors` (`self.Sphere`) (`self.Enemy`))))
    (`self.SpawnEnemy`)))

(fn `SpawnEnemy`
  (returns (Success :type Boolean))
  (if (`KismetArrayLibrary.Array_IsValidIndex` (`self.EnemyQueue`))
    (bind _returnvalue (`|SpawnActorFromClass` (`|GetArrayItem` (`self.EnemyQueue`)) (`self.GetTransform`) "AdjustIfPossibleButAlwaysSpawn" "OverrideRootScale" null null))
    (add `/Game/Jace/AI/SkyWatcharAI/BP_FlyingTurret.OnEnemyDestroyed` _returnvalue (`|CreateDelegate` :!event `OnEnemyDefeated`))
    (`KismetArrayLibrary.Array_Remove` (`self.EnemyQueue`))
    (`KismetSystemLibrary.K2_SetTimer` null "SpawnEnemy" 2.0)
    (return true)
    (else
      (return false))))

(fn `UserConstructionScript`)