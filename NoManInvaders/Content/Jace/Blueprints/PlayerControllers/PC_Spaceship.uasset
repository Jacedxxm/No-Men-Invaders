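; Player controller for the spaceship that adds the Enhanced Input mapping context, shows the cursor and creates the HUD on BeginPlay.
; Key 1 is a placeholder return to the main menu.
; Mouse-offset pitch/yaw steering with lerped roll is disconnected, leaving Tick empty.
; Helpers for that steering include CheckDeadZone, which eases input inside the dead zone, and an uncalled GetMousePosition variant with per-axis dead zones.
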(event `Key|One`
  (params (Key :type "Key Structure"))
  ;[1 1 1] Placeholder  Return to Menu
  (:`Pressed`
    (`GameplayStatics.OpenLevelBySoftObjectPtr` "/Game/Jace/Maps/scn_MainMenu.scn_MainMenu")))

(event `self.ReceiveBeginPlay`
  (bind _returnvalue (pcsubsystem `EnhancedInputLocalPlayerSubsystem` self))
  ;[1 1 1] Setup Inputs
  (`/Engine/EditorBlueprintResources/StandardMacros.IsValid` _returnvalue
    (:`Is Valid`
      (`EnhancedInputSubsystemInterface.AddMappingContext` _returnvalue "/Game/Jace/Blueprints/Inputs/IMC_Spaceship.IMC_Spaceship" 0 (struct))
      (set `self.bShowMouseCursor` true)
      (bind _returnvalue_2 (`|CreateWidget` "/Game/Jace/Blueprints/Widgets/WBP_HUD.WBP_HUD_C"))
      (`UserWidget.AddToViewport` _returnvalue_2 0))))

(event `self.ReceiveTick`
  (params (DeltaSeconds :type "Float (single-precision)"))
  ;[1 1 1] Mouse Position (TBF)
)

(fn `CheckDeadZone`
  (params (NewParam :type "Vector2D Structure"))
  (returns (NewParam1 :type "Vector2D Structure"))
  (if (> (`KismetMathLibrary.VSize2D` NewParam) (`KismetMathLibrary.VSize2D` (`KismetMathLibrary.MakeVector2D` (`self.Yaw Deadzone`) (`self.Pitch Deadzone`))))
    (if (!= (`self.Alpha`) 0.0)
      (bind _output_get (set `self.Alpha` (`KismetMathLibrary.FClamp` (- (`self.Alpha`) (* (`GameplayStatics.GetWorldDeltaSeconds`) (`self.AngularAccel`))))))
      (return (* (`KismetMathLibrary.Normal2D` NewParam) (`KismetMathLibrary.Lerp` (`KismetMathLibrary.VSize2D` NewParam) 0.0 _output_get)))
      (else
        (return NewParam)))
    (else
      (bind _output_get_2 (set `self.Alpha` (`KismetMathLibrary.FClamp` (+ (`self.Alpha`) (* (`GameplayStatics.GetWorldDeltaSeconds`) (`self.AngularAccel`))))))
      (return (* (`KismetMathLibrary.Normal2D` NewParam) (`KismetMathLibrary.Lerp` (`KismetMathLibrary.VSize2D` NewParam) 0.0 _output_get_2))))))

(fn `GetMousePosition_0`
  (locals (X :type "Float (double-precision)") (Y :type "Float (double-precision)"))
  (bind (_returnvalue_x _returnvalue_y) (`KismetMathLibrary.BreakVector2D` (/ (`WidgetLayoutLibrary.GetViewportSize`) 2.0)))
  (bind _returnvalue_x_2 (`KismetMathLibrary.BreakVector2D` (/ (`WidgetLayoutLibrary.GetViewportSize`) 2.0)))
  (bind _returnvalue (`WidgetLayoutLibrary.GetMousePositionOnViewport`))
  (bind (_returnvalue_x_3 _returnvalue_y_2) (`KismetMathLibrary.BreakVector2D` (- (* _returnvalue (`WidgetLayoutLibrary.GetViewportScale`)) (/ (`WidgetLayoutLibrary.GetViewportSize`) 2.0))))
  (bind _returnvalue_2 (`KismetMathLibrary.NormalizeToRange` (`KismetMathLibrary.Abs` _returnvalue_x_3) 0.0 _returnvalue_x_2))
  (if (<= _returnvalue_2 (`self.Yaw Deadzone`))
    (set `local.X` 0.0)
    (else
      (set `local.X` _returnvalue_2)))
  (bind _returnvalue_3 (`KismetMathLibrary.NormalizeToRange` (`KismetMathLibrary.Abs` _returnvalue_y_2) 0.0 _returnvalue_y))
  (if (<= _returnvalue_3 (`self.Pitch Deadzone`))
    (set `local.Y` 0.0)
    (else
      (set `local.Y` _returnvalue_3)))
  (set `self.MousePosition` (`KismetMathLibrary.MakeVector2D` (* (`local.X`) (`KismetMathLibrary.SignOfFloat` _returnvalue_x_3)) (* (* (`local.Y`) (`KismetMathLibrary.SignOfFloat` _returnvalue_y_2)) -1.0))))

(fn `UserConstructionScript`)