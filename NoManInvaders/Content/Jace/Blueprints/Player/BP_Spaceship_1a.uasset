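; Player spaceship pawn with thrust, vertical movement, smoothed roll, boost and twin mouse-aimed projectile launchers.
; Tick turns the ship by cursor offset from screen centre with an eased dead zone, widens FOV with speed and updates thruster Niagara spawn rates.
; A MoveCamera timeline blends spring arm length and pitch for first/third-person switching and boosting.
; A health component drives death, which destroys the ship and opens a paused menu.
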(event `EnhancedInput|/Game/Jace/Blueprints/Inputs/Actions/IA_Sprint`
  (params (ActionValue :type Boolean) (ElapsedSeconds :type "Float (double-precision)") (TriggeredSeconds :type "Float (double-precision)") (InputAction :type "InputAction Object Reference" :default "/Game/Jace/Blueprints/Inputs/Actions/IA_Sprint.IA_Sprint"))
  ;[1 1 1] Camera System
  ;;[1 0.1412 0.01151 0.5] Boost/Sprint (Placeholder)
  (:`Started`
    (`self.CurrentSpeedEqualZero`
      (:`true`
        (`ActorComponent.Activate` (`self.SpeedLines`) false)
        (set `FloatingPawnMovement.MaxSpeed` (`self.BoostedSpeed`) (`self.FloatingPawnMovement`))
        (set `FloatingPawnMovement.Acceleration` (`self.BoostedAcceleration`) (`self.FloatingPawnMovement`))
        (set `self.IsSprinting` true)
        (`self.IsFirst-Person`
          (:`true`
            (`self.MoveCamera` 0.0)
            (`self.ResetCamera`))
          (:`false`
            (`self.MoveCamera` (`self.Sprint Camera Arm Lenght`) (`self.ThirdPerson Camera Rotation`))
            (`self.ResetCamera`)))
        (set `self.IsSprinting` true))))
  (:`Canceled`
    (`ActorComponent.Deactivate` (`self.SpeedLines`) :!label _label)
    (set `FloatingPawnMovement.MaxSpeed` (`self.SP_BaseSpeed`) (`self.FloatingPawnMovement`))
    (set `FloatingPawnMovement.Acceleration` (`self.SP_BaseAcceleration`) (`self.FloatingPawnMovement`))
    (set `self.IsSprinting` false)
    (`self.IsFirst-Person`
      (:`true`
        (`self.MoveCamera` 0.0)
        (`self.ResetCamera`))
      (:`false`
        (`self.MoveCamera` 2000.0 (`self.ThirdPerson Camera Rotation`))
        (`self.ResetCamera`)))
    (set `self.IsSprinting` false))
  (:`Completed`
    (goto _label)))

(event `MoveCamera`
  (params (`Target Arm Lenght` :type "Float (double-precision)") (`Target Arm Rotation` :type "Float (double-precision)"))
  (bind _springarm (`self.SpringArm`))
  (bind _springarm_2 (`self.SpringArm`))
  (bind (_relativerotation_roll _relativerotation_pitch) (`KismetMathLibrary.BreakRotator` (`SceneComponent.RelativeRotation` _springarm)))
  ;[1 1 1] Camera System
  ;;[0.1354 1 0.7861 0.5] Camera Manager
  (set `self.Last Field Of View` (`CameraComponent.FieldOfView` (`self.Camera`)))
  (set `self.Last Arm Length` (`SpringArmComponent.TargetArmLength` _springarm))
  (set `self.Last Arm Rotation` _relativerotation_pitch)
  (bind (_direction _newtrack_0) (`Timeline|CameraMovement` :!label _label_2)
    (:`Update`
      (set `SpringArmComponent.TargetArmLength` (`KismetMathLibrary.Lerp` (`self.Last Arm Length`) `Target Arm Lenght` _newtrack_0) _springarm_2)
      (`SceneComponent.K2_SetRelativeRotation` _springarm_2 (`KismetMathLibrary.MakeRotator` 0.0 (`KismetMathLibrary.Lerp` (`self.Last Arm Rotation`) `Target Arm Rotation` _newtrack_0)) false false))))

(event `StopCamera`
  ;[1 1 1] Camera System
  ;;[0.1354 1 0.7861 0.5] Camera Manager
  (goto _label_2 :!via `Stop`))

(event `ResetCamera`
  ;[1 1 1] Camera System
  ;;[0.1354 1 0.7861 0.5] Camera Manager
  (goto _label_2 :!via `SetNewTime`))

(event `EnhancedInput|/Game/Jace/Blueprints/Inputs/Actions/IA_CameraSwitch`
  (params (ActionValue :type Boolean) (ElapsedSeconds :type "Float (double-precision)") (TriggeredSeconds :type "Float (double-precision)") (InputAction :type "InputAction Object Reference" :default "/Game/Jace/Blueprints/Inputs/Actions/IA_CameraSwitch.IA_CameraSwitch"))
  (bind _springarm (`self.SpringArm`))
  ;[1 1 1] Camera System
  ;;[1 0 0 0.613] Camera Switch
  (:`Started`
    (`/Engine/EditorBlueprintResources/StandardMacros.FlipFlop`
      (:`A`
        (set `SpringArmComponent.SocketOffset` (0.0 0.0 0.0) _springarm)
        (`self.MoveCamera` 0.0 (`self.FirstPerson Camera Rotation`))
        (`self.ResetCamera`)
        (set `self.First-Person` true)
        (if (`self.IsSprinting`)
          (`self.MoveCamera` 0.0)
          (`self.ResetCamera`)
          (else
            (`self.FirstPersonCamera`))))
      (:`B`
        (set `SpringArmComponent.SocketOffset` (`KismetMathLibrary.VLerp` (`SpringArmComponent.SocketOffset` _springarm) (0.0 0.0 200.0) 1.0) _springarm)
        (`self.MoveCamera` 2000.0 (`self.ThirdPerson Camera Rotation`))
        (`self.ResetCamera`)
        (set `self.First-Person` false)
        (if (`self.IsSprinting`)
          (`self.MoveCamera` 3000.0 (`self.ThirdPerson Camera Rotation`))
          (`self.ResetCamera`)
          (else
            (`self.ThirdPersonCamera`)))))))

(event `self.ReceiveBeginPlay`
  (bind _floatingpawnmovement (`self.FloatingPawnMovement`))
  ;[0.8367 0 1 0.408] Setup
  (set `SpringArmComponent.SocketOffset` (0.0 0.0 200.0) (`self.SpringArm`))
  (set `FloatingPawnMovement.MaxSpeed` (`self.SP_BaseSpeed`) _floatingpawnmovement)
  (set `FloatingPawnMovement.Acceleration` (`self.SP_BaseAcceleration`) _floatingpawnmovement)
  (set `self.CurrentSpeed` (`KismetMathLibrary.VSize` (`self.GetVelocity`)))
  (set `self.Default Camera FOV` (`CameraComponent.FieldOfView` (`self.Camera`)))
  (bind _returnvalue (`|CreateWidget` "/Game/Jace/Blueprints/Widgets/WBP_HUD.WBP_HUD_C"))
  (bind _output_get (set `self.HUD` _returnvalue))
  (`UserWidget.AddToViewport` _output_get 0))

(event `EnhancedInput|/Game/Jace/Blueprints/Inputs/Actions/IA_Move`
  (params (ActionValue :type "Vector Structure") (ElapsedSeconds :type "Float (double-precision)") (TriggeredSeconds :type "Float (double-precision)") (InputAction :type "InputAction Object Reference" :default "/Game/Jace/Blueprints/Inputs/Actions/IA_Move.IA_Move"))
  ;[0.3376 1 0 0.785] Base Movement
  (:`Triggered`
    (`self.AddMovementInput` (`self.GetActorForwardVector`) ActionValue_X)
    (`self.AddMovementInput` (`self.GetActorUpVector`) ActionValue_Z)))

(event `EnhancedInput|/Game/Jace/Blueprints/Inputs/Actions/IA_Roll`
  (params (ActionValue :type "Vector Structure") (ElapsedSeconds :type "Float (double-precision)") (TriggeredSeconds :type "Float (double-precision)") (InputAction :type "InputAction Object Reference" :default "/Game/Jace/Blueprints/Inputs/Actions/IA_Roll.IA_Roll"))
  ;[0.3376 1 0 0.785] Base Movement
  (:`Triggered`
    (set `self.Action Value Z` ActionValue_Z)))

(event `EnhancedInput|/Game/Jace/Blueprints/Inputs/Actions/IA_RealeseRoll`
  (params (ActionValue :type "Vector Structure") (ElapsedSeconds :type "Float (double-precision)") (TriggeredSeconds :type "Float (double-precision)") (InputAction :type "InputAction Object Reference" :default "/Game/Jace/Blueprints/Inputs/Actions/IA_RealeseRoll.IA_RealeseRoll"))
  ;[0.3376 1 0 0.785] Base Movement
  (:`Triggered`
    (set `self.Action Value Z` 0.0)))

(event `self.ReceiveTick`
  (params (DeltaSeconds :type "Float (single-precision)"))
  (bind _returnvalue (`GameplayStatics.GetWorldDeltaSeconds`))
  (bind _thrustermaxvelocity (`self.ThrusterMaxVelocity`))
  (bind (_locationx _locationy) (`PlayerController.GetMousePosition` (`GameplayStatics.GetPlayerController` 0)))
  (bind _returnvalue_2 (* (`WidgetLayoutLibrary.GetViewportSize`) 0.5))
  (bind (_newparam1_x _newparam1_y) (`KismetMathLibrary.BreakVector2D` (`self.CheckDeadZone` (/ (- (`KismetMathLibrary.MakeVector2D` _locationx _locationy) _returnvalue_2) _returnvalue_2))))
  ;[0 1 0.2685 0.476] Mouse Position + Actor Rotation
  (bind _output_get (set `self.Current Z Rotation` (`KismetMathLibrary.Lerp` (`self.Current Z Rotation`) (`self.Action Value Z`) (* (`self.RollSpeed`) (`GameplayStatics.GetWorldDeltaSeconds`)))))
  (`self.K2_AddActorLocalRotation` (`GameplayStatics.GetPlayerPawn` 0) (`KismetMathLibrary.MakeRotator` _output_get (* _newparam1_y (`self.Max Pitch Speed`) _returnvalue -1.0) (* _newparam1_x (`self.Max Yaw Speed`) _returnvalue)) false false)
  (set `CameraComponent.FieldOfView` (+ (`self.Default Camera FOV`) (`self.GetFOVIncrement`)) (`self.Camera`))
  (`NiagaraComponent.SetVariableFloat` (`self.Niagara1`) "SpawnRate" (+ (* (`self.ThrusterMovingVelocity`) (/ (`KismetMathLibrary.FClamp` (`KismetMathLibrary.VSize` (`self.GetVelocity`)) 0.0 _thrustermaxvelocity) _thrustermaxvelocity)) 0.0))
  (`NiagaraComponent.SetVariableFloat` (`self.Niagara3`) "SpawnRate" (+ (* (`self.ThrusterMovingVelocity`) (/ (`KismetMathLibrary.FClamp` (`KismetMathLibrary.VSize` (`self.GetVelocity`)) 0.0 _thrustermaxvelocity) _thrustermaxvelocity)) 0.0)))

(event `Key|LeftMouseButton`
  (params (Key :type "Key Structure"))
  (bind _bp_projectiglelaunchingcomponent1 (`self.BP_ProjectigleLaunchingComponent1`))
  ;[1 1 1] Shooting
  (:`Pressed`
    (`/Game/Jace/AI/Enemies/Components/BP_ProjectigleLaunchingComponent.LaunchProjectileAtLocation` (`self.BP_ProjectigleLaunchingComponent`) (+ (* (`.WorldDirection` (`PlayerController.DeprojectMousePositionToWorld` (`GameplayStatics.GetPlayerController` 0))) 140.0) (`SceneComponent.K2_GetComponentLocation` (`self.BP_ProjectigleLaunchingComponent`))))
    (`/Game/Jace/AI/Enemies/Components/BP_ProjectigleLaunchingComponent.LaunchProjectileAtLocation` _bp_projectiglelaunchingcomponent1 (+ (* (`.WorldDirection` (`PlayerController.DeprojectMousePositionToWorld` (`GameplayStatics.GetPlayerController` 0))) 140.0) (`SceneComponent.K2_GetComponentLocation` _bp_projectiglelaunchingcomponent1)))))

(event `self.BP_HealthSystemComponent.OnDead`
  ;[1 1 1] Death
  (`self.K2_DestroyActor`)
  (bind _returnvalue (`|CreateWidget` "/Game/Jace/Blueprints/Widgets/WBP_PauseMenu.WBP_PauseMenu_C" (`GameplayStatics.GetPlayerController` 0)))
  (`UserWidget.AddToViewport` _returnvalue 0)
  (`GameplayStatics.SetGamePaused` true))

(fn `CheckDeadZone`
  (params (InputPin :type "Vector2D Structure"))
  (returns (NewParam1 :type "Vector2D Structure"))
  (if (> (`KismetMathLibrary.VSize2D` InputPin) (`KismetMathLibrary.VSize2D` (`KismetMathLibrary.MakeVector2D` (`self.Yaw Deadzone`) (`self.Pitch Deadzone`))))
    (if (!= (`self.Alpha`) 0.0)
      (bind _output_get (set `self.Alpha` (`KismetMathLibrary.FClamp` (- (`self.Alpha`) (* (`GameplayStatics.GetWorldDeltaSeconds`) (`self.AngularAccel`))))))
      (return (* (`KismetMathLibrary.Normal2D` InputPin) (`KismetMathLibrary.Lerp` (`KismetMathLibrary.VSize2D` InputPin) 0.0 _output_get)))
      (else
        (return InputPin)))
    (else
      (bind _output_get_2 (set `self.Alpha` (`KismetMathLibrary.FClamp` (+ (`self.Alpha`) (* (`GameplayStatics.GetWorldDeltaSeconds`) (`self.AngularAccel`))))))
      (return (* (`KismetMathLibrary.Normal2D` InputPin) (`KismetMathLibrary.Lerp` (`KismetMathLibrary.VSize2D` InputPin) 0.0 _output_get_2))))))

(fn `GetFOVIncrement`
  (returns (ReturnValue :type "Float (double-precision)"))
  (bind _boostedspeed (`self.BoostedSpeed`))
  (return (* (`self.MovingFOV`) (/ (`KismetMathLibrary.FClamp` (`KismetMathLibrary.VSize` (`self.GetVelocity`)) 0.0 _boostedspeed) _boostedspeed))))

(fn `GetMousePosition`
  (locals (X :type "Float (double-precision)") (Y :type "Float (double-precision)"))
  (bind (_returnvalue_x _returnvalue_y) (`KismetMathLibrary.BreakVector2D` (/ (`WidgetLayoutLibrary.GetViewportSize`) 2.0)))
  (bind _returnvalue_x_2 (`KismetMathLibrary.BreakVector2D` (/ (`WidgetLayoutLibrary.GetViewportSize`) 2.0)))
  (bind _returnvalue (`WidgetLayoutLibrary.GetMousePositionOnViewport`))
  (bind (_returnvalue_x_3 _returnvalue_y_2) (`KismetMathLibrary.BreakVector2D` (- (* _returnvalue (`WidgetLayoutLibrary.GetViewportScale`)) (/ (`WidgetLayoutLibrary.GetViewportSize`) 2.0))))
  (bind _returnvalue_2 (`KismetMathLibrary.NormalizeToRange` (`KismetMathLibrary.Abs` _returnvalue_x_3) 0.0 _returnvalue_x_2))
  (if (<= _returnvalue_2 0.3)
    (set `local.X` 0.0)
    (else
      (set `local.X` _returnvalue_2)))
  (bind _returnvalue_3 (`KismetMathLibrary.NormalizeToRange` (`KismetMathLibrary.Abs` _returnvalue_y_2) 0.0 _returnvalue_y))
  (if (<= _returnvalue_3 0.3)
    (set `local.Y` 0.0)
    (else
      (set `local.Y` _returnvalue_3)))
  (set `self.MousePosition` (`KismetMathLibrary.MakeVector2D` (* (`local.X`) (`KismetMathLibrary.SignOfFloat` _returnvalue_x_3)) (* (* (`local.Y`) (`KismetMathLibrary.SignOfFloat` _returnvalue_y_2)) -1.0))))

(fn `UserConstructionScript`
  (`/Game/Jace/Blueprints/HealthSystem/BP_HealthSystemComponent.Setup Damageable Component` (`self.BP_HealthSystemComponent`) null (`self.MaxHealth`) (`self.Heatlh`) (`self.Widget`)))