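; BP_Spaceship is the player's flyable ship pawn, using FloatingPawnMovement for forward and vertical thrust.
; Each Tick it applies smoothed roll input plus pitch and yaw from the mouse's screen-center offset, eased through CheckDeadZone's dead zone.
; Sprint boosts speed, acceleration and FOV, while camera switch plays a timeline forward or backward to blend between third- and first-person views.
; An older GetMousePosition-based rotation path remains but never runs.
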(event `self.ReceiveBeginPlay`
  (bind _floatingpawnmovement (`self.FloatingPawnMovement`))
  ;[0.8367 0 1 0.408] Setup
  (set `FloatingPawnMovement.MaxSpeed` (`self.SP_BaseSpeed`) _floatingpawnmovement)
  (set `FloatingPawnMovement.Acceleration` (`self.SP_BaseAcceleration`) _floatingpawnmovement))

(event `EnhancedInput|/Game/Jace/Blueprints/Inputs/Actions/IA_Move`
  (params (ActionValue :type "Vector Structure") (ElapsedSeconds :type "Float (double-precision)") (TriggeredSeconds :type "Float (double-precision)") (InputAction :type "InputAction Object Reference" :default "/Game/Jace/Blueprints/Inputs/Actions/IA_Move.IA_Move"))
  ;[0.3376 1 0 0.785] Base Movement
  (:`Triggered`
    (`self.AddMovementInput` (`self.GetActorForwardVector`) ActionValue_X)
    (`self.AddMovementInput` (`self.GetActorUpVector`) ActionValue_Z)))

(event `EnhancedInput|/Game/Jace/Blueprints/Inputs/Actions/IA_Roll`
  (params (ActionValue :type "Vector Structure") (ElapsedSeconds :type "Float (double-precision)") (TriggeredSeconds :type "Float (double-precision)") (InputAction :type "InputAction Object Reference" :default "/Game/Jace/Blueprints/Inputs/Actions/IA_Roll.IA_Roll"))
  ;[0.3376 1 0 0.785] Base Movement
  (:`Triggered`
    (set `self.Action Value Z` ActionValue_Z)))

(event `EnhancedInput|/Game/Jace/Blueprints/Inputs/Actions/IA_RealeseRoll`
  (params (ActionValue :type "Vector Structure") (ElapsedSeconds :type "Float (double-precision)") (TriggeredSeconds :type "Float (double-precision)") (InputAction :type "InputAction Object Reference" :default "/Game/Jace/Blueprints/Inputs/Actions/IA_RealeseRoll.IA_RealeseRoll"))
  ;[0.3376 1 0 0.785] Base Movement
  (:`Triggered`
    (set `self.Action Value Z` 0.0)))

(event `self.ReceiveTick`
  (params (DeltaSeconds :type "Float (single-precision)"))
  (bind _returnvalue (`GameplayStatics.GetWorldDeltaSeconds`))
  (bind (_locationx _locationy) (`PlayerController.GetMousePosition` (`GameplayStatics.GetPlayerController` 0)))
  (bind _returnvalue_2 (* (`WidgetLayoutLibrary.GetViewportSize`) 0.5))
  (bind (_newparam1_x _newparam1_y) (`KismetMathLibrary.BreakVector2D` (`self.CheckDeadZone` (/ (- (`KismetMathLibrary.MakeVector2D` _locationx _locationy) _returnvalue_2) _returnvalue_2))))
  ;[1 1 1] P.
  (bind _output_get (set `self.Current Z Rotation` (`KismetMathLibrary.Lerp` (`self.Current Z Rotation`) (`self.Action Value Z`) (* (`self.RollSpeed`) (`GameplayStatics.GetWorldDeltaSeconds`)))))
  (`self.K2_AddActorLocalRotation` (`KismetMathLibrary.MakeRotator` _output_get (* _newparam1_y (`self.Max Pitch Speed`) _returnvalue -1.0) (* _newparam1_x (`self.Max Yaw Speed`) _returnvalue))))

(event `EnhancedInput|/Game/Jace/Blueprints/Inputs/Actions/IA_Sprint`
  (params (ActionValue :type Boolean) (ElapsedSeconds :type "Float (double-precision)") (TriggeredSeconds :type "Float (double-precision)") (InputAction :type "InputAction Object Reference" :default "/Game/Jace/Blueprints/Inputs/Actions/IA_Sprint.IA_Sprint"))
  (bind _floatingpawnmovement (`self.FloatingPawnMovement`))
  (bind _camera (`self.Camera`))
  ;[1 1 1] Boost/Sprint
  (:`Started`
    (set `FloatingPawnMovement.MaxSpeed` (`self.BoostedSpeed`) _floatingpawnmovement)
    (set `FloatingPawnMovement.Acceleration` (`self.BoostedAcceleration`) _floatingpawnmovement)
    (set `CameraComponent.FieldOfView` 110.0 _camera))
  (:`Canceled`
    (set `FloatingPawnMovement.MaxSpeed` (`self.SP_BaseSpeed`) _floatingpawnmovement :!label _label)
    (set `FloatingPawnMovement.Acceleration` (`self.SP_BaseAcceleration`) _floatingpawnmovement)
    (set `CameraComponent.FieldOfView` 90.0 _camera))
  (:`Completed`
    (goto _label)))

(event `EnhancedInput|/Game/Jace/Blueprints/Inputs/Actions/IA_CameraSwitch`
  (params (ActionValue :type Boolean) (ElapsedSeconds :type "Float (double-precision)") (TriggeredSeconds :type "Float (double-precision)") (InputAction :type "InputAction Object Reference" :default "/Game/Jace/Blueprints/Inputs/Actions/IA_CameraSwitch.IA_CameraSwitch"))
  ;[1 0.5265 0.1983] CameraSwitch
  (:`Started`
    (`/Engine/EditorBlueprintResources/StandardMacros.FlipFlop`
      (:`A`
        (`self.FPCamera`))
      (:`B`
        (`self.TPCamera`)))))

(event `FPCamera`
  ;[1 0.5265 0.1983] CameraSwitch
  (bind (_direction _transitiontime) (`Timeline|TransitionTime` :!label _label_2)
    (:`Update`
      (`SceneComponent.K2_SetWorldTransform` (`self.Camera`) (`KismetMathLibrary.TLerp` (`SceneComponent.K2_GetComponentToWorld` (`self.ThirdPersonCameraPosition`)) (`SceneComponent.K2_GetComponentToWorld` (`self.FirstPersonCameraPosition`)) _transitiontime) false false))))

(event `TPCamera`
  ;[1 0.5265 0.1983] CameraSwitch
  (goto _label_2 :!via `Reverse`))

(fn `CheckDeadZone`
  (params (NewParam :type "Vector2D Structure"))
  (returns (NewParam1 :type "Vector2D Structure"))
  (if (> (`KismetMathLibrary.VSize2D` NewParam) (`KismetMathLibrary.VSize2D` (`KismetMathLibrary.MakeVector2D` (`self.Yaw Deadzone`) (`self.Pitch Deadzone`))))
    (if (!= (`self.Alpha`) 0.0)
      (bind _output_get (set `self.Alpha` (`KismetMathLibrary.FClamp` (- (`self.Alpha`) (* (`GameplayStatics.GetWorldDeltaSeconds`) (`self.AngularAccel`))))))
      (return (* (`KismetMathLibrary.Normal2D` NewParam) (`KismetMathLibrary.Lerp` (`KismetMathLibrary.VSize2D` NewParam) 0.0 _output_get)))
      (else
        (return NewParam)))
    (else
      (bind _output_get_2 (set `self.Alpha` (`KismetMathLibrary.FClamp` (+ (`self.Alpha`) (* (`GameplayStatics.GetWorldDeltaSeconds`) (`self.AngularAccel`))))))
      (return (* (`KismetMathLibrary.Normal2D` NewParam) (`KismetMathLibrary.Lerp` (`KismetMathLibrary.VSize2D` NewParam) 0.0 _output_get_2))))))

(fn `GetMousePosition`
  (locals (X :type "Float (double-precision)") (Y :type "Float (double-precision)"))
  (bind (_returnvalue_x _returnvalue_y) (`KismetMathLibrary.BreakVector2D` (/ (`WidgetLayoutLibrary.GetViewportSize`) 2.0)))
  (bind _returnvalue_x_2 (`KismetMathLibrary.BreakVector2D` (/ (`WidgetLayoutLibrary.GetViewportSize`) 2.0)))
  (bind _returnvalue (`WidgetLayoutLibrary.GetMousePositionOnViewport`))
  (bind (_returnvalue_x_3 _returnvalue_y_2) (`KismetMathLibrary.BreakVector2D` (- (* _returnvalue (`WidgetLayoutLibrary.GetViewportScale`)) (/ (`WidgetLayoutLibrary.GetViewportSize`) 2.0))))
  (bind _returnvalue_2 (`KismetMathLibrary.NormalizeToRange` (`KismetMathLibrary.Abs` _returnvalue_x_3) 0.0 _returnvalue_x_2))
  (if (<= _returnvalue_2 (`self.Yaw Deadzone`))
    (set `local.X` 0.0)
    (else
      (set `local.X` _returnvalue_2)))
  (bind _returnvalue_3 (`KismetMathLibrary.NormalizeToRange` (`KismetMathLibrary.Abs` _returnvalue_y_2) 0.0 _returnvalue_y))
  (if (<= _returnvalue_3 (`self.Pitch Deadzone`))
    (set `local.Y` 0.0)
    (else
      (set `local.Y` _returnvalue_3)))
  (set `self.MousePosition` (`KismetMathLibrary.MakeVector2D` (* (`local.X`) (`KismetMathLibrary.SignOfFloat` _returnvalue_x_3)) (* (* (`local.Y`) (`KismetMathLibrary.SignOfFloat` _returnvalue_y_2)) -1.0))))

(fn `UserConstructionScript`)