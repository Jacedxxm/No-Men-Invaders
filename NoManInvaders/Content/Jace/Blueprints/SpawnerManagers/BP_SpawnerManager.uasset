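; Wave manager Blueprint meant to feed pooled enemies to BP_EnemySpawner actors, left mostly unwired.
; StartWave builds the pool count and loops up to EnemyMaxCount, but the random-spawner queue call is disconnected.
; BeginPlay is empty, and spawner gathering, wave increment and pool-size summing are unreachable.
; EndWave and EnterTransition are empty stubs, and GetEnemyFromPool has no selection logic.
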(event `self.ReceiveBeginPlay`)

(fn `BuildEnemyPool`
  (set `self.EnemyRemaining` (`self.GetPoolSize`)))

(fn `EndWave`)

(fn `EnterTransition`)

(fn `GetEnemyFromPool`
  (returns (Enemy :type "/Game/Jace/AI/FlyingAI/FlyingEnemies/AI_FlyingAI Class Reference")))

(fn `GetPoolSize`
  (returns (Sum :type Integer))
  (locals (LocalSum :type Integer)))

(fn `GetSpawners`)

(fn `NewWave`)

(fn `StartWave`
  (`self.BuildEnemyPool`)
  (for _ (range (`KismetMathLibrary.Min` (`self.GetPoolSize`) (`self.EnemyMaxCount`)))
    (bind _enemy (`self.GetEnemyFromPool`))))

(fn `UserConstructionScript`)