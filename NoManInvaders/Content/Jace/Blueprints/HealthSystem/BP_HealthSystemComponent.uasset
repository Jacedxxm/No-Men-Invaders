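; Health component that gives its owning actor damageable health and a floating or attached health bar widget.
; Setup on BeginPlay stores the owner, health values and bar; TakeDamageViaComponent subtracts damage, refreshes the bar, prints debug text and calls OnDead at zero or below.
; The WBP_HealthBar progress shows the health ratio, staying visible permanently or hiding after a delay following a hit.
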(event `self.ReceiveBeginPlay`
  (`self.Setup Damageable Component` (`self.GetOwner`) (`self.MaxHealth`) (`self.Health`) (`self.HealthBar`))
  (if (`self.ShowHealthBarAllTime`)
    (`SceneComponent.SetVisibility` (`self.HealthBar`) true false)))

(event `Setup Damageable Component`
  (params (OwningActor :type "Actor Object Reference") (MaxHealth :type "Float (double-precision)") (Health :type "Float (double-precision)") (HealthBar :type "WidgetComponent Object Reference"))
  (set `self.OwningActor` OwningActor)
  (set `self.MaxHealth` MaxHealth)
  (set `self.Health` Health)
  (set `self.HealthBar` HealthBar))

(event `TakeDamageViaComponent`
  (params (DamageAmount :type "Float (double-precision)"))
  (bind _output_get (set `self.Health` (- (`self.Health`) DamageAmount)))
  (`self.Update Healthbar`)
  (if (<= (`self.Health`) 0.0)
    (`KismetSystemLibrary.PrintString` "Dead")
    (`self.OnDead`)
    (else
      (`KismetSystemLibrary.PrintString` (`KismetStringLibrary.Concat_StrStr` "Hit_  " (`KismetStringLibrary.Conv_DoubleToString` DamageAmount) "Health_  " (`KismetStringLibrary.Conv_DoubleToString` _output_get))))))

(event `Update Healthbar`
  (bind _healthbar (`self.HealthBar`))
  (`SceneComponent.SetVisibility` (`self.HealthBar`) true false)
  (bind _aswbp_health_bar (cast `/Game/Jace/Blueprints/HealthSystem/Widgets/WBP_HealthBar` (`WidgetComponent.GetUserWidgetObject` (`self.HealthBar`))))
  (`ProgressBar.SetPercent` (`/Game/Jace/Blueprints/HealthSystem/Widgets/WBP_HealthBar.ProgressBar_189` _aswbp_health_bar) (/ (`self.Health`) (`self.MaxHealth`)))
  (if (`self.ShowHealthBarAllTime`)
    (`SceneComponent.SetVisibility` _healthbar true false)
    (else
      (`KismetSystemLibrary.Delay` (`self.VisibilityTime`))
      (`SceneComponent.SetVisibility` _healthbar false false))))