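; BP_Asteroid is an asteroid actor that randomizes the look of its five mesh components.
; The construction script gives each component a random static mesh from the Asteroids array.
; It also sets a random whole-number relative scale on each axis independently, allowing stretched, varied shapes.
; No seeded stream is used, so the result re-rolls whenever construction reruns.
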(fn `UserConstructionScript`
  (bind _returnvalue (`KismetMathLibrary.Conv_IntToDouble` (`KismetMathLibrary.RandomIntegerInRange` 1 10)))
  (for _array_element (`|MakeArray` (`self.Asteroid1`) (`self.Asteroid2`) (`self.Asteroid3`) (`self.Asteroid4`) (`self.Asteroid`))
    (`StaticMeshComponent.SetStaticMesh` _array_element (`KismetArrayLibrary.Array_Random` (`self.Asteroids`)))
    (`SceneComponent.SetRelativeScale3D` _array_element (`KismetMathLibrary.MakeVector` _returnvalue _returnvalue _returnvalue))))